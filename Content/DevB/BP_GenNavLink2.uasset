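; Smart nav link that makes a BP_TestCharacter agent vault to the link destination when reached, unless a montage is already playing.
; It sets three motion warping targets at the start, a raised midpoint and the destination, all facing the travel direction, then plays a zombie vault montage.
; Flying mode and disabled capsule collision carry the vault until montage completion restores walking and collision.
; Debug text and spheres mark each vault.
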(event EventSmartLinkReached
  (params (Agent :type Actor%20Object%20Reference) (Destination :type Vector :default "0, 0, 0"))
  (bind _returnvalue (Transformation|GetActorLocation Agent))
  (bind (_x _y) (Math|Vector|BreakVector Destination))
  (bind (_x_2 _y_2) (Math|Vector|BreakVector _returnvalue))
  (bind _returnvalue_2 (- Destination _returnvalue))
  (bind _returnvalue_3 (/ _returnvalue_2 2.0))
  (bind _returnvalue_4 (+ _returnvalue _returnvalue_3 "0.000000,0.000000,110.000000"))
  (bind _asbp_test_character (Utilities|Casting|CastToBP_TestCharacter Agent))
  (if (not (Class|AnimInstance|IsAnyMontagePlaying (Components|SkeletalMesh|GetAnimInstance (Variables|/Script/Engine.Character|GetMesh _asbp_test_character))))
    (Variables|Default|SetNewVar (Math|Rotator|FindLookatRotation (Math|Vector|MakeVector _x_2 _y_2 0.0) (Math|Vector|MakeVector _x _y 0.0)))
    (Pawn|Components|CharacterMovement|SetMovementMode (Variables|/Script/Engine.Character|GetCharacterMovement _asbp_test_character) "MOVE_Flying" 0)
    (Collision|SetCollisionEnabled (Variables|/Script/Engine.Character|GetCapsuleComponent _asbp_test_character) "NoCollision")
    (Class|MotionWarpingComponent|AddorUpdateWarpTargetfromLocationandRotation (Variables|/Game/Enemy/Blueprint/BP_TestCharacter.BP_TestCharacter_C|GetMotionWarping _asbp_test_character) "1" _returnvalue (Variables|Default|GetNewVar))
    (Class|MotionWarpingComponent|AddorUpdateWarpTargetfromLocationandRotation (Variables|/Game/Enemy/Blueprint/BP_TestCharacter.BP_TestCharacter_C|GetMotionWarping _asbp_test_character) "2" _returnvalue_4 (Variables|Default|GetNewVar))
    (Class|MotionWarpingComponent|AddorUpdateWarpTargetfromLocationandRotation (Variables|/Game/Enemy/Blueprint/BP_TestCharacter.BP_TestCharacter_C|GetMotionWarping _asbp_test_character) "3" Destination (Variables|Default|GetNewVar))
    (Animation|Montage|PlayMontage (Variables|/Script/Engine.Character|GetMesh _asbp_test_character) "/Game/Enemy/ZombieAsset/Mannequin_Animation/Parkour/ZombieIP_Vault_L_Montage.ZombieIP_Vault_L_Montage" 0.7
      (:then
        (Development|PrintString "Vault")
        (Rendering|Debug|DrawDebugSphere _returnvalue 3e+01 12 "(R=0.000000,G=1.000000,B=0.288715,A=1.000000)" 1e+01)
        (Rendering|Debug|DrawDebugSphere _returnvalue_4 3e+01 12 "(R=1.000000,G=0.000000,B=0.882851,A=1.000000)" 1e+01)
        (Rendering|Debug|DrawDebugSphere Destination 3e+01 12 "(R=1.000000,G=0.099890,B=0.000000,A=1.000000)" 1e+01))
      (:OnCompleted
        (Collision|SetCollisionEnabled (Variables|/Script/Engine.Character|GetCapsuleComponent _asbp_test_character) "QueryAndPhysics")
        (Pawn|Components|CharacterMovement|SetMovementMode (Variables|/Script/Engine.Character|GetCharacterMovement _asbp_test_character) "MOVE_Walking" 0)))))