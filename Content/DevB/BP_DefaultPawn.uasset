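; BP_DefaultPawn is a pawn that triggers a rifle gunshot noise where the player looks, apparently for testing noise reporting.
; Pressing 1 traces along the Visibility channel from the player camera's forward direction.
; On a hit, PlaySoundAndReportNoise plays the rifle cue and reports noise at the impact point, with the pawn as instigator.
; A separate ReportNoiseEvent node is left unconnected, and the default events are empty.
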(event EventBeginPlay)

(event Collision|EventActorBeginOverlap
  (params (OtherActor :type Actor%20Object%20Reference)))

(event EventTick
  (params (DeltaSeconds :type Float%20%28single-precision%29)))

(event Input|KeyboardEvents|1
  (params (Key :type Key%20Structure :default "None"))
  (bind _returnvalue (Game|GetPlayerCameraManager 0))
  (bind _returnvalue_2 (Camera|GetCameraLocation _returnvalue))
  (:Pressed
    (bind (_outhit _returnvalue_3) (Collision|LineTraceByChannel _returnvalue_2 (+ _returnvalue_2 (* (Math|Vector|GetForwardVector (Camera|GetCameraRotation _returnvalue)) 5e+04)) "TraceTypeQuery1" false 0 "None"))
    (if _returnvalue_3
      (Class|OutBreakGlobal|PlaySoundandReportNoise "/Game/Weapons/Ranged/Rifle/Sounds/Cue/CUE_RifleB_Fire_End_ST03_Cue.CUE_RifleB_Fire_End_ST03_Cue" (.Location (Collision|BreakHitResult _outhit)) self))))

(fn ConstructionScript)