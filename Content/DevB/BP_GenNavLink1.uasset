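; BP_GenNavLink1 is a smart nav link that launches a BP_TestCharacter across to the link's destination when the agent reaches it.
; It computes a custom-arc projectile velocity, adds extra upward boost, and calls LaunchCharacter with full velocity override.
; An IsUsing flag blocks further use and is not cleared here; the character receives a pointer to the link.
; A debug sphere and printed message show the destination.
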(event EventSmartLinkReached
  (params (Agent :type Actor%20Object%20Reference) (Destination :type Vector :default "0, 0, 0"))
  (if (not (Variables|Default|GetbIsUsing))
    (bind _asbp_test_character (Utilities|Casting|CastToBP_TestCharacter Agent))
    (Variables|Default|SetbIsUsing true)
    (Variables|/Game/Enemy/Blueprint/BP_TestCharacter.BP_TestCharacter_C|SetNavLinkPtr _asbp_test_character self)
    (Rendering|Debug|DrawDebugSphere Destination 3e+01 12 "(R=1.000000,G=1.000000,B=1.000000,A=1.000000)" 1e+01)
    (Development|PrintString (Utilities|String|ToString(Vector) Destination) true true "(R=0.000000,G=0.660000,B=1.000000,A=1.000000)" 1e+01)
    (bind _outlaunchvelocity (Game|SuggestProjectileVelocityCustomArc (Transformation|GetActorLocation Agent) Destination 0.0 0.5))
    (Character|LaunchCharacter _asbp_test_character (+ _outlaunchvelocity "0.000000,0.000000,300.000000") true true)))