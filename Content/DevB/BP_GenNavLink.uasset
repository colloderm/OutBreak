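; BP_GenNavLink is a nav link Blueprint that makes characters jump across when they reach its smart link.
; SmartLinkReached computes an arc velocity from the agent to the destination, adds extra upward velocity, and launches the character with it.
; It also prints the offset to the destination.
; A disconnected branch would instead launch downward-bound agents with a short hop, ragdoll their mesh and make their capsule ignore pawns.
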(event EventSmartLinkReached
  (params (Agent :type Actor%20Object%20Reference) (Destination :type Vector :default "0, 0, 0"))
  (bind _returnvalue (Transformation|GetActorLocation Agent))
  (bind _as캐릭터 (Utilities|Casting|CastToCharacter Agent))
  (Development|PrintString (Utilities|String|ToString(Vector) (- Destination _returnvalue)))
  (bind _outlaunchvelocity (Game|SuggestProjectileVelocityCustomArc _returnvalue Destination 0.0 0.5))
  (Character|LaunchCharacter _as캐릭터 (+ _outlaunchvelocity "0.000000,0.000000,300.000000") true true))