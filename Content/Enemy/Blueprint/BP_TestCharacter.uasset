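; Test enemy character that plays physics-based hit reactions and recovers from ragdoll.
; Point damage prints the bone name and, except at the pelvis, stops movement, blends physics below that bone via a timeline, and applies a delayed impulse.
; Tick caches the simulated mesh's position while falling, then after a delay disables physics, moves the actor there and resets the mesh.
; Tick also clears the nav link's in-use flag whenever the character isn't falling.
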(event EventBeginPlay)

(event Collision|EventActorBeginOverlap
  (params (OtherActor :type Actor%20Object%20Reference)))

(event EventTick
  (params (DeltaSeconds :type Float%20%28single-precision%29))
  (Utilities|FlowControl|Sequence
    (:then_0
      (if (Physics|IsSimulatingPhysics (Variables|Character|GetMesh) "None")
        (if (AI|Components|NavMovement|IsFalling (Variables|Character|GetCharacterMovement))
          (Variables|Default|SetCacheMeshPos (Transformation|GetWorldLocation (Variables|Character|GetMesh)))
          (else
            (Utilities|FlowControl|RetriggerableDelay 1.0)
            (Physics|SetSimulatePhysics (Variables|Character|GetMesh) false)
            (Collision|SetCollisionEnabled (Variables|Character|GetMesh) "NoCollision")
            (Collision|SetCollisionResponsetoChannel (Variables|Collision|GetCapsuleComponent) "ECC_Pawn" "ECR_Block")
            (Transformation|SetActorLocation (Variables|Default|GetCacheMeshPos) false false)
            (Transformation|SetRelativeTransform (Variables|Character|GetMesh) (Math|Transform|MakeTransform "0.000000,0.000000,-90.000000" "0.000000,-90.000000,0.000000") false false)))))
    (:then_1
      (Variables|Default|GetNavLinkPtr
        (:then
          (if (not (AI|Components|NavMovement|IsFalling (Variables|Character|GetCharacterMovement)))
            (Variables|/Game/DevB/BP_GenNavLink1.BP_GenNavLink1_C|SetbIsUsing (Variables|Default|GetNavLinkPtr) false)))
        (:else)))))

(event Game|Damage|EventPointDamage
  (params (Damage :type Float%20%28single-precision%29) (DamageType :type Damage%20Type%20Object%20Reference) (HitLocation :type Vector :default "0, 0, 0") (HitNormal :type Vector :default "0, 0, 0") (HitComponent :type Primitive%20Component%20Object%20Reference) (BoneName :type Name :default "None") (ShotFromDirection :type Vector :default "0, 0, 0") (InstigatedBy :type Controller%20Object%20Reference) (DamageCauser :type Actor%20Object%20Reference) (HitInfo :type Hit%20Result%20Structure%20%28by%20ref%29))
  (Rendering|Debug|DrawDebugString HitLocation (Utilities|String|ToString(Name) BoneName) 0 "(R=1.000000,G=1.000000,B=1.000000,A=1.000000)" 2.0)
  (if (!= BoneName "pelvis")
    (Variables|Default|SetBone%20Name BoneName)
    (if (not (Variables|Default|GetIsHit))
      (Variables|Default|SetIsHit true)
      (Components|Movement|StopMovementImmediately (Variables|Character|GetCharacterMovement))
      (Utilities|FlowControl|Sequence
        (:then_0
          (bind _새_트랙_0 (Timeline|타임라인 PlayFromStart)
            (:Update
              (Variables|Default|SetBlendWeight _새_트랙_0)
              (Class|SkeletalMeshComponent|SetAllBodiesBelowSimulatePhysics (Variables|Character|GetMesh) (Variables|Default|GetBone%20Name) true true)
              (Class|SkeletalMeshComponent|SetAllBodiesBelowPhysicsBlendWeight (Variables|Character|GetMesh) (Variables|Default|GetBone%20Name) (Variables|Default|GetBlendWeight) false true))
            (:Finished
              (Class|SkeletalMeshComponent|SetAllBodiesPhysicsBlendWeight (Variables|Character|GetMesh) 0.0 false)
              (Class|SkeletalMeshComponent|SetAllBodiesSimulatePhysics (Variables|Character|GetMesh) false)
              (Variables|Default|SetIsHit false))))
        (:then_1
          (Utilities|FlowControl|Delay 0.1)
          (Physics|AddImpulse (Variables|Character|GetMesh) (* HitNormal 1e+04) (Variables|Default|GetBone%20Name) true))))))

(fn ConstructionScript)