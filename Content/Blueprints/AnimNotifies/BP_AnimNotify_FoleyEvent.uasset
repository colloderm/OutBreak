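; Anim notify that triggers a gameplay-tagged foley sound from an animation, skipped while the animation is blending out.
; It first offers the event to the owner's OBFootstepComponent at the foot socket matching Side.
; If that is absent or returns false, AC_FoleyEvents plays it with side, volume and pitch, falling back to a 2D sound from DefaultBank without that component.
; The notify's name shows the tag's last segment.
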(fn ReceivedNotify
  (params (MeshComp :type Skeletal%20Mesh%20Component%20Object%20Reference) (Animation :type Anim%20Sequence%20Base%20Object%20Reference) (EventReference :type Anim%20Notify%20Event%20Reference%20Structure%20%28by%20ref%29))
  (bind _returnvalue (Components|GetOwner MeshComp))
  (bind _returnvalue_2 (Components|GetOwner MeshComp))
  (bind _returnvalue_3 (Actor|GetComponentbyClass _returnvalue "/Game/Weapons/Audio/Foley/AC_FoleyEvents.AC_FoleyEvents_C"))
  (bind _returnvalue_4 (Actor|GetComponentbyClass _returnvalue_2 "/Script/OutBreak.OBFootstepComponent"))
  (if (not (Class|AnimNotifyLibrary|IsBlendingOut EventReference))
    (Utilities|IsValid _returnvalue_4
      (:Is%20Valid
        (bind _returnvalue_5 (Class|OBFootstepComponent|PlayFootstepfromFoley _returnvalue_4 MeshComp (Variables|Default|GetEvent) (Utilities|Select :Index (Variables|Default|GetSide) :NewEnumerator4 "foot_l" :NewEnumerator0 "foot_l" :NewEnumerator2 "foot_r")))
        (if (not _returnvalue_5)
          (Utilities|IsValid _returnvalue_3 :!label _label
            (:Is%20Valid
              (Default|PlayFoleyEvent _returnvalue_3 (Variables|Default|GetEvent) (Utilities|Struct|MakeS_FoleyEventParams (Variables|Default|GetSide) (Variables|Default|GetVolumeMultiplier) (Variables|Default|GetPitchMultiplier)))
              (return true))
            (:Is%20Not%20Valid
              (Audio|PlaySound2D (.Sound (Default|GetSoundfromFoleyEvent (Variables|Default|GetDefaultBank) (Variables|Default|GetEvent))) (Variables|Default|GetVolumeMultiplier) (Variables|Default|GetPitchMultiplier) 0.0 0 0)))))
      (:Is%20Not%20Valid
        (goto _label)))))

(fn GetNotifyName
  (return (Utilities|String|ToString(Text) (Utilities|Text|FormatText "FoleyEvent: {Type}" (.RightS (Utilities|String|Split (GameplayTags|GetDebugStringfromGameplayTag (Variables|Default|GetEvent)) "." "IgnoreCase" "FromEnd"))))))