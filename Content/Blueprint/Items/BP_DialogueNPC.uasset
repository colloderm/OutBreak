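; BP_DialogueNPC is an interactable NPC that runs a table-driven conversation and can hand out a starting loadout.
; Interact opens WBP_Dialogue through the player controller, binds its dialogue action event, and starts from the configured table and node.
; The basic-equipment action gives an assault rifle and pistol via OBLoadoutSubsystem only when the loadout is empty, then jumps the dialogue to a given or already-have branch.
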(event Custom|HandleAction
  (params (Action :type EOBDialogueAction%20Enum :default "None"))
  (bind _returnvalue (Subsystems|GetOBLoadoutSubsystem))
  (bind _activedialogue (Variables|Default|GetActiveDialogue))
  (switch Utilities|FlowControl|Switch|SwitchonEOBDialogueAction Action
    (:GiveStarterKit
      (if (Class|OBLoadoutSubsystem|IsEmpty _returnvalue)
        (Class|OBLoadoutSubsystem|SetWeapon _returnvalue "Primary" "/Game/Blueprint/Weapons/BP_AssaultRifle.BP_AssaultRifle_C")
        (Class|OBLoadoutSubsystem|SetWeapon _returnvalue "Secondary" "/Game/Blueprint/Weapons/BP_Pistol.BP_Pistol_C")
        (Class|OBDialogueWidget|GotoNode _activedialogue "AfterGive")
        (else
          (Class|OBDialogueWidget|GotoNode _activedialogue "AlreadyHave"))))))

(event EventBeginPlay)

(event Collision|EventActorBeginOverlap
  (params (OtherActor :type Actor%20Object%20Reference)))

(event EventTick
  (params (DeltaSeconds :type Float%20%28single-precision%29)))

(event EventInteract
  (params (PC :type OB%20Player%20Controller%20Object%20Reference))
  (bind _returnvalue (Class|OBPlayerController|OpenInteractionWidget PC "/Game/UI/NPC/WBP_Dialogue.WBP_Dialogue_C"))
  (bind _asobdialogue_widget (Utilities|Casting|CastToOBDialogueWidget _returnvalue))
  (bind _output_get (Variables|Default|SetActiveDialogue _asobdialogue_widget))
  (EventDispatchers|BindEventtoOnDialogueAction _output_get (delegate Custom|HandleAction))
  (Class|OBDialogueWidget|StartDialogue _output_get (Variables|Default|GetDialogueTable) (Variables|Default|GetStartNode)))

(fn ConstructionScript)