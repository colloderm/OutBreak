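; BP_Flare is a flare that climbs like a firework, then bursts into sparks.
; Each tick it offsets along its up vector by Speed, while a launch sound plays at spawn.
; After a short delay it stops, spawns a spark emitter and explosion sound, removes its Niagara component, then destroys itself.
; Both sounds report noise tagged "Flare".
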(event EventBeginPlay
  (Class|OutBreakGlobal|PlaySoundandReportNoise "/Game/Sound/Firework_peu_front_3sec_Cue.Firework_peu_front_3sec_Cue" (Transformation|GetActorLocation) 0 "Flare")
  (Utilities|FlowControl|Delay 3.0)
  (Utilities|FlowControl|Sequence
    (:then_0
      (Variables|Default|SetSpeed 0.0)
      (Effects|SpawnEmitteratLocation "/Game/Realistic_Starter_VFX_Pack_Vol2/Particles/Sparks/P_Sparks_G.P_Sparks_G" (Transformation|GetActorLocation) "-180.000000,0.000000,0.000000" "3.000000,3.000000,3.000000")
      (Class|OutBreakGlobal|PlaySoundandReportNoise "/Game/Sound/Firework_Explosion_Cue.Firework_Explosion_Cue" (Transformation|GetActorLocation) 0 "Flare")
      (Utilities|FlowControl|Delay 2.0)
      (Actor|DestroyActor))
    (:then_1
      (Utilities|FlowControl|Delay 0.9)
      (Components|DestroyComponent (Variables|Default|GetNiagara)))))

(event Collision|EventActorBeginOverlap
  (params (OtherActor :type Actor%20Object%20Reference)))

(event EventTick
  (params (DeltaSeconds :type Float%20%28single-precision%29))
  (Transformation|AddActorWorldOffset (* (Transformation|GetActorUpVector) (Variables|Default|GetSpeed))))

(fn ConstructionScript)